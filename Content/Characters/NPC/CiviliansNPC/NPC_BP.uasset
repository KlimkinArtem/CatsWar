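; NPC_BP is a civilian NPC with a randomized cat color that speeds up when it perceives the player shooting.
; On BeginPlay it picks a random material from CatColors and applies it to mesh slots 3 through 7.
; An AI perception update from a ThirdPersonCharacter with the Shoot tag raises its max walk speed.
; The file contains no movement logic and never lowers the speed again.
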(event OnTargetPerceptionUpdated(AIPerception)
  (params (Actor :type Actor%20Object%20Reference) (Stimulus :type AI%20Stimulus%20Structure))
  (Utilities|Casting|CastToThirdPersonCharacter Actor)
  (switch name (.Tag (Utilities|Struct|BreakAIStimulus Stimulus))
    (:Shoot
      (Variables|/Script/Engine.CharacterMovementComponent|SetMaxWalkSpeed (Variables|Character|GetCharacterMovement) 8e+02))))

(event EventBeginPlay
  (Variables|Default|SetCat%20color%20mat (Utilities|Array|Get(acopy) (Variables|Default|GetCat%20colors) (Math|Random|RandomInteger 5)))
  (for _index (range 3 7)
    (Rendering|Material|SetMaterial (Variables|Character|GetMesh) _index (Variables|Default|GetCat%20color%20mat))))

(fn ConstructionScript)