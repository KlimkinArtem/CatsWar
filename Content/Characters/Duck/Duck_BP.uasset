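; Duck character Blueprint that handles melee punch attacks and damage reaction animations.
; Attack plays a random punch montage behind a DoOnce gate, which Resetattack reopens to allow the next punch.
; Attackstart calls MeleAttack to perform the hit check, while DamageAnim plays a random damage montage.
; BeginPlay only calls the parent, and a leftover Test event prints a greeting.
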(event Custom|Attack
  (Utilities|FlowControl|DoOnce false
    (:Completed
      (Animation|PlayAnimMontage (Utilities|Array|Get(acopy) (Variables|Default|GetPunch) (Math|Random|RandomInteger 4)) 1.0 "None"))))

(event Custom|Reset%20attack
  (Utilities|FlowControl|DoOnce false) ; enters at Reset
)

(event Custom|Attack%20start
  (Class|PatrollingAICPP|MeleAttack 5e+01 10 false))

(event Custom|DamageAnim
  (Animation|PlayAnimMontage (Utilities|Array|Get(acopy) (Variables|Default|GetDamage) (Math|Random|RandomInteger 2)) 1.0 "None"))

(event Custom|Test
  (Development|PrintString "Hello"))

(event EventBeginPlay
  (|CallParentFunction))

(event Collision|EventActorBeginOverlap
  (params (OtherActor :type Actor%20Object%20Reference))
  (|CallParentFunction OtherActor) ; This node is disabled and will not be called.\nDrag off pins to build functionality.
)

(event EventTick
  (params (DeltaSeconds :type Float%20%28single-precision%29))
  (|CallParentFunction DeltaSeconds) ; This node is disabled and will not be called.\nDrag off pins to build functionality.
)

(fn ConstructionScript
  (|CallParentFunction))